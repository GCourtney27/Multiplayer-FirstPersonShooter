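; MP18 weapon Blueprint, a child class that relies on inherited variables such as the weapon mesh and projectile type.
; BeginPlay runs the parent logic, casts ProjectileType to the .45 ACP projectile and caches the first-person player.
; Its fire and stop-fire interface events are empty.
; A disconnected, never-run chain holds camera-trace firing: interface damage on hit, then a projectile spawned at the muzzle, aimed at the impact point or trace end.
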(event `self.ReceiveBeginPlay`
  (`parent.ReceiveBeginPlay`)
  (`|ExecutionSequence`
    (:`then_0`
      (bind _asbp_projectile_45acp (castclass `/Game/Blueprints/Projectiles/BP_Projectile_45acp` (`self.ProjectileType`)))
      (set `self.ProjectileType` _asbp_projectile_45acp))
    (:`then_1`
      (bind _asbp_first_person (cast `/Game/Blueprints/FirstPersonCharacter/BP_FirstPerson` (`GameplayStatics.GetPlayerCharacter` 0)))
      (set `self.Player_Ref` _asbp_first_person))))

(event `/Game/Blueprints/Weapons/BPI_Weapon.IFireWeapon`)

(event `/Game/Blueprints/Weapons/BPI_Weapon.IStopFireWeapon`)

(fn `UserConstructionScript`
  (`parent.UserConstructionScript`))