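; BP_Weapon is a weapon Blueprint that drives a dynamic crosshair for the player.
; On BeginPlay it creates the WBCrosshair widget, adds it to the viewport and hides it until EnableCrosshair is called.
; Each Tick it maps player character 0's velocity magnitude to the widget's CrosshairSpread, clamped between idle and walk limits.
; EnableCrosshair and DisableCrosshair toggle the widget's visibility.
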(event `self.ReceiveBeginPlay`
  (`|ExecutionSequence`
    (:`then_0`
      (bind _returnvalue (`|CreateWidget` "/Game/UI/Gameplay/DynamicCrossHair.WBCrosshair_C"))
      (bind _output_get (set `self.DynamicCrosshair_Widget` _returnvalue))
      (`UserWidget.AddToViewport` _output_get 0)
      (`self.DisableCrosshair`))))

(event `self.ReceiveTick`
  (params (DeltaSeconds :type "Float (single-precision)"))
  (set `/Game/UI/Gameplay/DynamicCrossHair.crosshair_spread` (`KismetMathLibrary.MapRangeClamped` (`KismetMathLibrary.VSize` (`self.GetVelocity` (`GameplayStatics.GetPlayerCharacter` 0))) (`self.InA`) (`self.InB`) (`self.CrosshairMaxIdleSpread`) (`self.CrosshairMaxWalkSpread`)) (`self.DynamicCrosshair_Widget`)))

(fn `DisableCrosshair`
  (`Widget.SetVisibility` (`self.DynamicCrosshair_Widget`) "Hidden"))

(fn `EnableCrosshair`
  (`Widget.SetVisibility` (`self.DynamicCrosshair_Widget`) "Visible"))

(fn `UserConstructionScript`)