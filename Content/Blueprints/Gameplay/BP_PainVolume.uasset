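; BP_PainVolume is a volume that periodically damages the first-person player while they are inside it.
; Overlap events with BP_FirstPerson toggle the IsPlayerInVolume flag.
; Tick runs through a Delay of DamageDelay, which throttles DamagePlayer into a repeating interval.
; DamagePlayer checks the flag, gets player character 0 and sends it damage through BPI_Damageable, naming the volume as hitter.
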(event `self.ReceiveActorBeginOverlap`
  (params (OtherActor :type "Actor Object Reference"))
  (cast `/Game/Blueprints/FirstPersonCharacter/BP_FirstPerson` OtherActor)
  (set `self.IsPlayerInVolume` true))

(event `self.ReceiveActorEndOverlap`
  (params (OtherActor :type "Actor Object Reference"))
  (cast `/Game/Blueprints/FirstPersonCharacter/BP_FirstPerson` OtherActor)
  (set `self.IsPlayerInVolume` false))

(event `self.ReceiveTick`
  (params (DeltaSeconds :type "Float (single-precision)"))
  (`KismetSystemLibrary.Delay` (`self.DamageDelay`))
  (`self.DamagePlayer`))

(fn `DamagePlayer`
  (if (`self.IsPlayerInVolume`)
    (bind _asbp_first_person (cast `/Game/Blueprints/FirstPersonCharacter/BP_FirstPerson` (`GameplayStatics.GetPlayerCharacter` 0)))
    (if (`KismetSystemLibrary.DoesImplementInterface` _asbp_first_person "/Game/Blueprints/FirstPersonCharacter/BPI_Damageable.BPI_Damageable_C")
      (message `/Game/Blueprints/FirstPersonCharacter/BPI_Damageable.IRecieveDamage` _asbp_first_person (`self.Damage`) self))))

(fn `UserConstructionScript`)