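; BP_TestTarget is a simple damageable test target actor that tracks health and can be destroyed.
; A sphere component prints a hit message on overlap but does not apply damage itself.
; A RecieveDamage event subtracts the incoming amount from Health, then at zero or below clears IsAlive, destroys the actor and prints a death message.
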(event `self.Sphere.OnComponentBeginOverlap`
  (params (OverlappedComponent :type "PrimitiveComponent Object Reference") (OtherActor :type "Actor Object Reference") (OtherComp :type "PrimitiveComponent Object Reference") (OtherBodyIndex :type Integer) (bFromSweep :type Boolean) (SweepResult :type "HitResult Structure (by ref)"))
  (`KismetSystemLibrary.PrintString` "Target Hit"))

(event `/Game/Blueprints/FirstPersonCharacter/BPI_Damageable.RecieveDamage`
  (params (Damage :type "Float (single-precision)") (Hitter :type "Actor Object Reference"))
  (`|ExecutionSequence`
    (:`then_0`
      (set `self.Health` (- (`self.Health`) Damage)))
    (:`then_1`
      (if (<= (`self.Health`) 0.0)
        (set `self.IsAlive` false)
        (`self.K2_DestroyActor`)
        (`KismetSystemLibrary.PrintString` "Target Dead")))))

(fn `UserConstructionScript`)