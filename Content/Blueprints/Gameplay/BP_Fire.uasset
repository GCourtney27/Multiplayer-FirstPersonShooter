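; BP_Fire is a fire hazard actor that flickers its light and damages the first-person character on contact.
; A LightFlicker timeline starts on BeginPlay and scales the point light's intensity by LightIntensity.
; When BP_FirstPerson begins overlapping the box collider, the actor sends a single damage message through BPI_Damageable, so damage does not repeat while the overlap lasts.
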(event `self.ReceiveBeginPlay`
  (bind (_direction _flicker) (`Timeline|LightFlicker`)
    (:`Update`
      (`LightComponent.SetIntensity` (`self.PointLight`) (* _flicker (`self.lightIntensity`))))))

(event `self.BoxCollider.OnComponentBeginOverlap`
  (params (OverlappedComponent :type "PrimitiveComponent Object Reference") (OtherActor :type "Actor Object Reference") (OtherComp :type "PrimitiveComponent Object Reference") (OtherBodyIndex :type Integer) (bFromSweep :type Boolean) (SweepResult :type "HitResult Structure (by ref)"))
  (bind _asbp_first_person (cast `/Game/Blueprints/FirstPersonCharacter/BP_FirstPerson` OtherActor))
  (if (`KismetSystemLibrary.DoesImplementInterface` _asbp_first_person "/Game/Blueprints/FirstPersonCharacter/BPI_Damageable.BPI_Damageable_C")
    (message `/Game/Blueprints/FirstPersonCharacter/BPI_Damageable.IRecieveDamage` _asbp_first_person (`self.Damage`) self)))

(event `self.BoxCollider.OnComponentEndOverlap`
  (params (OverlappedComponent :type "PrimitiveComponent Object Reference") (OtherActor :type "Actor Object Reference") (OtherComp :type "PrimitiveComponent Object Reference") (OtherBodyIndex :type Integer)))

(fn `UserConstructionScript`)