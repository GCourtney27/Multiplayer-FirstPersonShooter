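; Camera manager actor that runs the deploy screen, switching the player between a tabletop overhead camera and the first-person character.
; On BeginPlay it binds to the player's death dispatcher, creates the DeployScreen widget and shows it over the tabletop view.
; Death returns to that view with movement and look input ignored.
; The widget's deploy event blends back to the character with a sound, hides the UI and respawns the player.
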(event `self.ReceiveBeginPlay`
  (`|ExecutionSequence`
    (:`then_0`
      ;[1 1 1] Register Death Event Dispatcher
      (bind _asbp_first_person (cast `/Game/Blueprints/FirstPersonCharacter/BP_FirstPerson` (`GameplayStatics.GetPlayerCharacter` 0)))
      (add `/Game/Blueprints/FirstPersonCharacter/BP_FirstPerson.DeathDispatcher` _asbp_first_person (delegate `SendPlayerToOverHead`)))
    (:`then_1`
      ;[1 1 1] Create the UI for the Deploy Screen
      (bind _returnvalue (`|CreateWidget` "/Game/UI/Gameplay/DeployScreen.DeployScreen_C"))
      (bind _output_get (set `self.DeployHUD` _returnvalue))
      (`UserWidget.AddToViewport` _output_get 0))
    (:`then_2`
      ;[1 1 1] Register Deploy Character Event Dispatcher
      (add `/Game/UI/Gameplay/DeployScreen.DeployCharacter` (`self.DeployHUD`) (delegate `DeployCharacter`)))
    (:`then_3`
      (`self.ApplyDeployHUD`))
    (:`then_4`
      (`self.TransitionCameraToTabletop`))))

(event `SendPlayerToOverHead`
  ;[1 1 1] Register Death Event Dispatcher
  (`|ExecutionSequence`
    (:`then_0`
      (`self.TransitionCameraToTabletop`))
    (:`then_1`
      (`self.ApplyDeployHUD`))))

(event `DeployCharacter`
  ;[1 1 1] Register Deploy Character Event Dispatcher
  (`|ExecutionSequence`
    (:`then_0`
      (`self.TransitionCameraFromTabletop`))
    (:`then_1`
      (`self.RemoveDeployHUD`))
    (:`then_2`
      (bind _asbp_first_person (cast `/Game/Blueprints/FirstPersonCharacter/BP_FirstPerson` (`GameplayStatics.GetPlayerCharacter` 0)))
      (`/Game/Blueprints/FirstPersonCharacter/BP_FirstPerson.Respawn Player` _asbp_first_person))))

(fn `ApplyDeployHUD`
  ;[1 1 1] Apply HUD
  (`Widget.SetVisibility` (`self.DeployHUD`) "Visible")
  (set `PlayerController.bShowMouseCursor` true (`GameplayStatics.GetPlayerController` 0)))

(fn `RemoveDeployHUD`
  (`Widget.SetVisibility` (`self.DeployHUD`) "Hidden")
  (set `PlayerController.bShowMouseCursor` false (`GameplayStatics.GetPlayerController` 0)))

(fn `TransitionCameraFromTabletop`
  (bind _returnvalue (`GameplayStatics.GetPlayerController` 0))
  ;[1 1 1] Respawn
  (`GameplayStatics.PlaySound2D` "/Game/Audio/Deploy_Transition_In_02.Deploy_Transition_In_02" 1.0 1.0 0.0 null null)
  (`PlayerController.SetViewTargetWithBlend` _returnvalue (`GameplayStatics.GetPlayerCharacter` 0) 1.0 "VTBlend_EaseInOut" 1.0 false)
  (`Controller.ResetIgnoreMoveInput` _returnvalue)
  (`Controller.ResetIgnoreLookInput` _returnvalue))

(fn `TransitionCameraToTabletop`
  (bind _returnvalue (`GameplayStatics.GetPlayerController` 0))
  ;[1 1 1] To overhead
  (`GameplayStatics.PlaySound2D` "/Game/Audio/SquadSpawn_Transition.SquadSpawn_Transition" 1.0 1.0 0.0 null null)
  (`PlayerController.SetViewTargetWithBlend` _returnvalue (`ActorComponent.GetOwner` (`self.TableTop_Camera`)) 1.0 "VTBlend_EaseInOut" 3.0 false)
  (`Controller.SetIgnoreMoveInput` _returnvalue true)
  (`Controller.SetIgnoreLookInput` _returnvalue true))

(fn `UserConstructionScript`)