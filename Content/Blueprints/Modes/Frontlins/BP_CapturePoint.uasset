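; Capture point for the Frontlines mode that builds team scores while active and occupied.
; Box overlaps read the BP_FirstPerson team (1 is friendly, otherwise enemy) and set one presence flag per side, without counting occupants.
; Tick adds delta time times a point multiplier for each present side and copies totals to GM_FPS_Frontlines.
; The enemy increment writes its total into the game mode's FriendlyScore, as the friendly one does.
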(event `self.ReceiveBeginPlay`)

(event `self.ReceiveTick`
  (params (DeltaSeconds :type "Float (single-precision)"))
  (set `self.Time` DeltaSeconds)
  (if (`self.IsActive`)
    (`|ExecutionSequence`
      (:`then_0`
        (if (`self.FriendlyInCaptureZone`)
          (`self.IncrementFriendlyScore`)))
      (:`then_1`
        (if (`self.EnemyInCaptureZone`)
          (`self.IncrementEnemyScore`))))))

(event `self.Box.OnComponentBeginOverlap`
  (params (OverlappedComponent :type "PrimitiveComponent Object Reference") (OtherActor :type "Actor Object Reference") (OtherComp :type "PrimitiveComponent Object Reference") (OtherBodyIndex :type Integer) (bFromSweep :type Boolean) (SweepResult :type "HitResult Structure (by ref)"))
  (bind _asbp_first_person (cast `/Game/Blueprints/FirstPersonCharacter/BP_FirstPerson` OtherActor))
  (if (== (`/Game/Blueprints/FirstPersonCharacter/BP_FirstPerson.Team` _asbp_first_person) 1)
    (set `self.FriendlyInCaptureZone` true)
    (else
      (set `self.EnemyInCaptureZone` true))))

(event `self.Box.OnComponentEndOverlap`
  (params (OverlappedComponent :type "PrimitiveComponent Object Reference") (OtherActor :type "Actor Object Reference") (OtherComp :type "PrimitiveComponent Object Reference") (OtherBodyIndex :type Integer))
  (bind _asbp_first_person (cast `/Game/Blueprints/FirstPersonCharacter/BP_FirstPerson` OtherActor))
  (if (== (`/Game/Blueprints/FirstPersonCharacter/BP_FirstPerson.Team` _asbp_first_person) 1)
    (set `self.FriendlyInCaptureZone` false)
    (else
      (set `self.EnemyInCaptureZone` false))))

(fn `IncrementEnemyScore`
  (bind _output_get (set `self.EnemyScore` (+ (`self.EnemyScore`) (* (`self.PointMultiplier`) (`self.Time`)))))
  (bind _asgm_fps_frontlines (cast `/Game/Blueprints/GameModes/GM_FPS_Frontlines` (`GameplayStatics.GetGameMode`))
    (:`then`
      (set `/Game/Blueprints/GameModes/GM_FPS_Frontlines.FriendlyScore` _output_get _asgm_fps_frontlines))
    (:`CastFailed`
      (`KismetSystemLibrary.PrintString` "Failed to cast GM in enemy score increment"))))

(fn `IncrementFriendlyScore`
  (bind _output_get (set `self.FriendlyScore` (+ (`self.FriendlyScore`) (* (`self.PointMultiplier`) (`self.Time`)))))
  (bind _asgm_fps_frontlines (cast `/Game/Blueprints/GameModes/GM_FPS_Frontlines` (`GameplayStatics.GetGameMode`))
    (:`then`
      (set `/Game/Blueprints/GameModes/GM_FPS_Frontlines.FriendlyScore` _output_get _asgm_fps_frontlines))
    (:`CastFailed`
      (`KismetSystemLibrary.PrintString` "Failed to cast GM in friendly score increment"))))

(fn `UserConstructionScript`)