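; AI controller for BP_AI_Master enemies that patrols waypoints and attacks the player once an enemy is found.
; Patrol walks the pawn's waypoint list back and forth with pauses.
; A looping CheckEnemy timer polls the pawn's alive and detection flags, stopping on death or triggering OnHunt.
; OnHunt moves toward the player and, after a delay, fires a muzzle line trace that damages BP_FirstPerson.
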(event `self.ReceiveBeginPlay`
  (bind _asbp_ai_master (cast `/Game/Blueprints/AI/BP_AI_Master` (`self.K2_GetPawn`)))
  (set `self.AI_Base_Ref` _asbp_ai_master)
  (set `self.Waypoints` (`/Game/Blueprints/AI/BP_AI_Master.Waypoint` _asbp_ai_master))
  (bind _returnvalue (`KismetSystemLibrary.K2_SetTimer` null "CheckEnemy" 0.3 true))
  (set `self.CleanTimer` _returnvalue)
  (`KismetSystemLibrary.Delay` 2.0)
  (`|AIMoveTo` _asbp_ai_master (0.0 0.0 0.0) (`|GetArrayItem` (`self.Waypoints`) (`self.CurrentWaypoint`))
    (:`OnSuccess`
      (`KismetSystemLibrary.Delay` 3.0)
      (`self.Patroling`))))

(event `Patroling`
  (if (not (`self.FoundEnamy`))
    (if (`self.WalkBack`)
      (`/Engine/EditorBlueprintResources/StandardMacros.DecrementInt` (`self.CurrentWaypoint`)
        (:`  `
          (`|AIMoveTo` null (0.0 0.0 0.0) (`|GetArrayItem` (`self.Waypoints`) (`self.CurrentWaypoint`))
            (:`OnSuccess`
              (if (<= (`self.CurrentWaypoint`) 0)
                (set `self.WalkBack` false))))))
      (else
        (`/Engine/EditorBlueprintResources/StandardMacros.IncrementInt` (`self.CurrentWaypoint`)
          (:`  `
            (`|AIMoveTo` null (0.0 0.0 0.0) (`|GetArrayItem` (`self.Waypoints`) (`self.CurrentWaypoint`))
              (:`OnSuccess`
                (if (>= (`self.CurrentWaypoint`) (- (`KismetArrayLibrary.Array_Length` (`self.Waypoints`)) 1))
                  (set `self.WalkBack` true))))))))
    (`KismetSystemLibrary.Delay` 4.0)
    (`self.Patroling`)))

(event `OnHunt`
  (`|AIMoveTo` null (0.0 0.0 0.0) (`GameplayStatics.GetPlayerCharacter` 0) 1000.0
    (:`then`
      (`KismetSystemLibrary.Delay` 2.0)
      (`self.Fire`))))

(event `CheckEnemy`
  (bind _ai_base_ref (`self.AI_Base_Ref`))
  (if (not (`/Game/Blueprints/AI/BP_AI_Master.IsAlive` _ai_base_ref))
    (`KismetSystemLibrary.K2_ClearAndInvalidateTimerHandle` (`self.CleanTimer`))
    (`self.StopMovement`)
    (else
      (bind _output_get (set `self.FoundEnamy` (`/Game/Blueprints/AI/BP_AI_Master.EnemyFound` _ai_base_ref)))
      (if _output_get
        (`self.OnHunt`)))))

(event `Fire`
  (bind _sk_weapon (`/Game/Blueprints/Weapons/BP_Weapon.SK_Weapon` (`/Game/Blueprints/AI/BP_AI_Master.WeaponBP` (`self.AI_Base_Ref`))))
  (bind _returnvalue (`SceneComponent.GetSocketLocation` _sk_weapon "Muzzle"))
  (`GameplayStatics.PlaySoundAtLocation` "/Game/Audio/Misc/45_ACP_sound_effect.45_ACP_sound_effect" (`self.K2_GetActorLocation` (`ActorComponent.GetOwner` (`self.ActionsComp`))) (struct) 1.0 1.0 0.0 null null null)
  (bind (_outhit _returnvalue_2) (`KismetSystemLibrary.LineTraceSingle` :`Start` _returnvalue :`End` (+ _returnvalue (* (`KismetMathLibrary.GreaterGreater_VectorRotator` (`SceneComponent.GetForwardVector` _sk_weapon) (struct :`Yaw` 90.0 :`Roll` -30.0)) 15000.0)) :`TraceChannel` "TraceTypeQuery1" :`bTraceComplex` true :`TraceColor` (struct :`G` 0.031513 :`B` 1.0 :`A` 1.0)))
  (if true
    (bind (_bblockinghit _binitialoverlap _time _distance _location _impactpoint _normal _impactnormal _physmat _hitactor _hitcomponent _hitbonename _hititem _faceindex _tracestart _traceend) (`GameplayStatics.BreakHitResult` _outhit))
    (if (`KismetSystemLibrary.DoesImplementInterface` _hitactor "/Game/Blueprints/AI/BPI_TakeDamage.BPI_TakeDamage_C")
      (bind _asbp_first_person (cast `/Game/Blueprints/FirstPersonCharacter/BP_FirstPerson` _hitactor))
      (`/Game/Blueprints/FirstPersonCharacter/BP_FirstPerson.IRecieveDamage` _asbp_first_person 0.1 null))
    (`|SpawnActorFromClass` "/Game/Blueprints/Projectiles/BP_Projectile_45acp.BP_Projectile_45acp_C" (`KismetMathLibrary.MakeTransform` (0.0 0.0 0.0) (`KismetMathLibrary.FindLookAtRotation` (`SceneComponent.GetSocketLocation` (`/Game/Blueprints/Weapons/BP_Weapon.SK_Weapon` (`/Game/Blueprints/AI/BP_AI_Master.WeaponBP` (`self.AI_Base_Ref`))) "Muzzle") (`KismetMathLibrary.SelectVector` _impactpoint _traceend _returnvalue_2))) "Undefined" "OverrideRootScale" null null)))

(fn `UserConstructionScript`)