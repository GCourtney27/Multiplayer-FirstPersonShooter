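; BP_AI_Master is an AI character, apparently a base for armed enemies, with health, a HUD widget and ragdoll death.
; On BeginPlay it fills health, sets itself as the AI_HUD owner and attaches a spawned MP18 to its mesh's weapon socket.
; ITakeDamage kills instantly on head hits; other hits reduce health and flag EnemyFound.
; Survivors set EquipWeapon, while death enables mesh physics, disables capsule collision and hides the widget.
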(event `self.ReceiveBeginPlay`
  (set `self.CurrentHealth` (`self.MaxHealth`))
  (bind _asai_hud (cast `/Game/Blueprints/AI/AI_HUD` (`WidgetComponent.GetUserWidgetObject` (`self.Widget`))))
  (set `/Game/Blueprints/AI/AI_HUD.Owner` self _asai_hud)
  (bind _returnvalue (`|SpawnActorFromClass` "/Game/Blueprints/Weapons/BP_Weapon_MP18.BP_Weapon_MP18_C" (`KismetMathLibrary.MakeTransform` (0.0 0.0 0.0)) "Undefined" "OverrideRootScale" null null))
  (bind _output_get (set `self.WeaponBP` _returnvalue))
  (`self.K2_AttachToComponent` _output_get (`self.Mesh`) "Weapon_Attach" "SnapToTarget" "SnapToTarget" "KeepRelative" true))

(event `/Game/Blueprints/AI/BPI_TakeDamage.ITakeDamage`
  (params (BoneName :type Name) (Damage :type "Float (single-precision)"))
  (bind _currenthealth (`self.CurrentHealth`))
  (if (== BoneName "Head")
    (set `self.CurrentHealth` 0.0)
    (else
      (set `self.EnemyFound` true)
      (set `self.CurrentHealth` (- _currenthealth Damage))))
  (if (<= _currenthealth 0.0)
    (set `self.IsAlive` false)
    (`SkeletalMeshComponent.SetAllBodiesSimulatePhysics` (`self.Mesh`) true)
    (`PrimitiveComponent.SetCollisionEnabled` (`self.CapsuleComponent`) "NoCollision")
    (`SceneComponent.SetVisibility` (`self.Widget`) false false)
    (else
      (set `self.EquipWeapon` true))))

(fn `UserConstructionScript`)