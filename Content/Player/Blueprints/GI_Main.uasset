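; Game instance that manages the front-end menus and multiplayer session hosting and joining.
; InitMenus creates and caches the main, multiplayer, host and search widgets, adding all to the viewport with only the main visible; Show events reveal each.
; CreateLobby creates an advanced session tagged with the server name, LAN unless Steam, then opens MP_Outskirts; JoinSession joins a given search result.
; Menu music switching logic is present but disconnected.
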(event `InitMainMenu`
  ;[1 1 1] Init Main Menu
  (`/Engine/EditorBlueprintResources/StandardMacros.IsValid` (`self.MainMenu`)
    (:`Is Valid`
      _)
    (:`Is Not Valid`
      (bind _returnvalue (`|CreateWidget` "/Game/UI/Munus/MainMenu.MainMenu_C" (`GameplayStatics.GetPlayerController` 0)))
      (bind _output_get (set `self.MainMenu` _returnvalue))))
  (`UserWidget.AddToViewport` _output_get 0))

(event `InitHostGameMenu`
  ;[1 1 1] Init Host Game Menu
  (`/Engine/EditorBlueprintResources/StandardMacros.IsValid` (`self.HostGame`)
    (:`Is Valid`
      _)
    (:`Is Not Valid`
      (bind _returnvalue (`|CreateWidget` "/Game/UI/Munus/CreateGame.CreateGame_C" (`GameplayStatics.GetPlayerController` 0)))
      (bind _output_get (set `self.HostGame` _returnvalue))))
  (`UserWidget.AddToViewport` _output_get 0)
  (`Widget.SetVisibility` _output_get "Hidden"))

(event `InitMenus`
  ;[1 1 1] Load all menus into memory
  (`|ExecutionSequence`
    (:`then_0`
      (`self.InitMainMenu`))
    (:`then_1`
      (`self.InitMultiplayerMenu`))
    (:`then_2`
      (`self.InitHostGameMenu`))
    (:`then_3`
      (`self.InitSearchGamesMenu`))))

(event `InitMultiplayerMenu`
  ;[1 1 1] Init Multplayer Menu
  (`/Engine/EditorBlueprintResources/StandardMacros.IsValid` (`self.Multiplyer`)
    (:`Is Valid`
      _)
    (:`Is Not Valid`
      (bind _returnvalue (`|CreateWidget` "/Game/UI/Munus/MultiplayerMenu.MultiplayerMenu_C" (`GameplayStatics.GetPlayerController` 0)))
      (bind _output_get (set `self.Multiplyer` _returnvalue))))
  (`UserWidget.AddToViewport` _output_get 0)
  (`Widget.SetVisibility` _output_get "Hidden"))

(event `InitSearchGamesMenu`
  ;[1 1 1] Init Seach Games Manu
  (`/Engine/EditorBlueprintResources/StandardMacros.IsValid` (`self.SearchGames`)
    (:`Is Valid`
      _)
    (:`Is Not Valid`
      (bind _returnvalue (`|CreateWidget` "/Game/UI/Munus/SearchGames.SearchGames_C" (`GameplayStatics.GetPlayerController` 0)))
      (bind _output_get (set `self.SearchGames` _returnvalue))))
  (`UserWidget.AddToViewport` _output_get 0)
  (`Widget.SetVisibility` _output_get "Hidden"))

(event `ShowMainMenu`
  ;[1 1 1] Redirect to Main menu
  (`Widget.SetVisibility` (`self.MainMenu`) "Visible"))

(event `ShowMultipayerMenu`
  ;[1 1 1] Redirect to Multiplayer menu
  (`Widget.SetVisibility` (`self.Multiplyer`) "Visible"))

(event `ShowHostGameMenu`
  ;[1 1 1] Redirect to Host Game menu
  (`Widget.SetVisibility` (`self.HostGame`) "Visible"))

(event `ShowSearchGameMenu`
  ;[1 1 1] Redirect to Search Game menu
  (`Widget.SetVisibility` (`self.SearchGames`) "Visible"))

(event `CreateLobby`
  (params (isSteamGame :type Boolean) (ServerName :type Text))
  ;[1 1 1] Launch Level
  (set `self.InputServerName` ServerName)
  (`CreateSessionCallbackProxyAdvanced.CreateAdvancedSession` (`|MakeArray` (`AdvancedSessionsLibrary.MakeLiteralSessionPropertyString` "servername" (`KismetTextLibrary.Conv_TextToString` (`self.InputServerName`)))) (`GameplayStatics.GetPlayerController` 0) 100 0 (not isSteamGame)
    (:`OnSuccess`
      (`GameplayStatics.OpenLevel` "MP_Outskirts" true "listen"))
    (:`OnFailure`
      (`KismetSystemLibrary.PrintString` "Failed to create session"))))

(event `JoinSession`
  (params (SessionToJoin :type "BlueprintSessionResult Structure"))
  ;[1 1 1] Join Session (Called from Game BP)
  (`JoinSessionCallbackProxy.JoinSession` (`GameplayStatics.GetPlayerController` 0) SessionToJoin
    (:`OnFailure`
      (`KismetSystemLibrary.PrintString` "Failed to join session"))))